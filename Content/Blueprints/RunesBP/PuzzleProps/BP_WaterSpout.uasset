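; BP_WaterSpout is a short-lived actor that sprays water from the player character for three seconds before destroying itself.
; A fast looping timer repeatedly spawns small, scaled-down BP_WaterStream actors slightly above the player's location, matching the player's rotation.
; Each spawned stream's Sphere receives an impulse along the player's forward vector, so the spray follows wherever the character moves and faces.
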(event `self.ReceiveBeginPlay`
  (`KismetSystemLibrary.K2_SetTimerDelegate` (delegate `Spawn Water Particles`) 0.1 true)
  (`KismetSystemLibrary.Delay` 3.0)
  (`self.K2_DestroyActor`))

(event `Spawn Water Particles`
  (bind _returnvalue (`GameplayStatics.GetPlayerCharacter` 0))
  (bind _returnvalue_2 (`|SpawnActorFromClass` "/Game/Blueprints/RunesBP/PuzzleProps/BP_WaterStream.BP_WaterStream_C" (`KismetMathLibrary.MakeTransform` (+ (`self.K2_GetActorLocation` _returnvalue) (0.0 0.0 40.0)) (`self.K2_GetActorRotation` _returnvalue) (0.05 0.05 0.05)) "Undefined" "OverrideRootScale" null null))
  (`PrimitiveComponent.AddImpulse` (`/Game/Blueprints/RunesBP/PuzzleProps/BP_WaterStream.Sphere` _returnvalue_2) (* (`SceneComponent.GetForwardVector` (`Actor.RootComponent` _returnvalue)) 150.0) "None" false))

(fn `UserConstructionScript`)