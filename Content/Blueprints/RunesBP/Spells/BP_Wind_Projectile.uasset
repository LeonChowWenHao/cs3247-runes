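; BP_Wind_Projectile is a wind spell projectile that pushes nearby physics objects away on impact.
; Each tick it sweeps itself forward along its scene component's forward vector at a fixed per-frame step, so speed depends on frame rate.
; On hit it fires a RadialForce impulse and destroys itself, and the Destroyed event plays a sound and spawns an explosion particle at its location.
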(event `self.ReceiveDestroyed`
  (bind _returnvalue (`self.K2_GetActorLocation`))
  ;[1 1 1] On destroy event, play sound and spawn emitter
  (`GameplayStatics.PlaySoundAtLocation` null _returnvalue (struct) 1.0 1.0 0.0 null null null)
  (`GameplayStatics.SpawnEmitterAtLocation` "/Game/Effects/Particles/Explosion/P_NeonExplosion.P_NeonExplosion" _returnvalue))

(event `self.ReceiveTick`
  (params (DeltaSeconds :type "Float (single-precision)"))
  ;[1 1 1] Forward movement
  (`self.K2_AddActorWorldOffset` (* (`SceneComponent.GetForwardVector` (`self.Scene`)) 25.0) true))

(event `self.ReceiveHit`
  (params (MyComp :type "PrimitiveComponent Object Reference") (Other :type "Actor Object Reference") (OtherComp :type "PrimitiveComponent Object Reference") (bSelfMoved :type Boolean) (HitLocation :type "Vector Structure") (HitNormal :type "Vector Structure") (NormalImpulse :type "Vector Structure") (Hit :type "HitResult Structure (by ref)"))
  ;[1 1 1] Fire impulse on hit
  (`RadialForceComponent.FireImpulse` (`self.RadialForce`))
  (`self.K2_DestroyActor`))

(fn `UserConstructionScript`)