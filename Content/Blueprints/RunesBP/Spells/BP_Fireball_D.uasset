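; BP_Fireball_D is a fireball spell projectile that burns obstructions and deactivates key switches.
; Tick moves the Sphere a fixed step along its local X axis, without sweep or delta-time scaling.
; A component hit calls Burn on a BP_Obstruction or Deactivate on a BP_Key_Switch, then destroys the fireball whatever was struck.
; A timer set on BeginPlay also destroys it after a few seconds.
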(event `self.ReceiveBeginPlay`
  (`KismetSystemLibrary.K2_SetTimerDelegate` (delegate `Expire`) 5.0))

(event `Expire`
  (`self.K2_DestroyActor` :!label _label))

(event `self.Sphere.OnComponentHit`
  (params (HitComponent :type "PrimitiveComponent Object Reference") (OtherActor :type "Actor Object Reference") (OtherComp :type "PrimitiveComponent Object Reference") (NormalImpulse :type "Vector Structure") (Hit :type "HitResult Structure (by ref)"))
  (bind _asbp_obstruction (cast `/Game/Blueprints/RunesBP/PuzzleProps/BP_Obstruction` OtherActor)
    (:`then`
      (`/Game/Blueprints/RunesBP/PuzzleProps/BP_Obstruction.Burn` _asbp_obstruction 2)
      (goto _label))
    (:`CastFailed`
      (bind _asbp_key_switch (cast `/Game/Blueprints/RunesBP/PuzzleProps/BP_Key_Switch` OtherActor)
        (:`then`
          (`/Game/Blueprints/RunesBP/PuzzleProps/BP_Key_Switch.Deactivate` _asbp_key_switch)
          (goto _label))
        (:`CastFailed`
          (goto _label))))))

(event `self.ReceiveTick`
  (params (DeltaSeconds :type "Float (single-precision)"))
  (`SceneComponent.K2_AddLocalOffset` (`self.Sphere`) (10.0 0.0 0.0) false false))

(fn `UserConstructionScript`)