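; Physics fan actor that blows physics objects and the player along its up axis with a simulated airflow.
; While anything overlaps the Range box, sized and offset in the construction script, Tick fires a grid of line traces upward.
; Each hit gets a randomised force scaled by distance and surface angle.
; Living players receive it through CharacterMovement to keep control; dead players and simulating components at the impact point.
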(event `self.ReceiveTick`
  (params (DeltaSeconds :type "Float (single-precision)"))
  (bind _returnvalue (`self.GetActorUpVector`))
  (bind _returnvalue_2 (`self.GetTransform`))
  (bind _pushforce (`self.PushForce`))
  (bind _linetracespacing (`self.LineTraceSpacing`))
  (if (> (`KismetArrayLibrary.Array_Length` (`PrimitiveComponent.GetOverlappingComponents` (`self.Range`))) 0)
    ;[1 1 1] Calculate position and number of ray traces based on 'RangeX', 'RangeY' and 'LineTraceSpacing'
    (for _index (range (+ (`KismetMathLibrary.FTrunc` (/ (`self.RangeX`) (`self.LineTraceSpacing`))) 1))
      (for _index_2 (range (+ (`KismetMathLibrary.FTrunc` (/ (`self.RangeY`) (`self.LineTraceSpacing`))) 1))
        (bind _returnvalue_3 (`KismetMathLibrary.MakeVector` (- (* _index _linetracespacing) (/ (`self.RangeY`) 2.0)) (- (* _index_2 _linetracespacing) (/ (`self.RangeX`) 2.0))))
        (bind (_outhit _returnvalue_4) (`KismetSystemLibrary.LineTraceSingle` :`Start` (`KismetMathLibrary.TransformLocation` _returnvalue_2 _returnvalue_3) :`End` (`KismetMathLibrary.TransformLocation` _returnvalue_2 (+ _returnvalue_3 (`KismetMathLibrary.MakeVector` 0.0 0.0 (* (`self.RangeZ`) 2.0)))) :`TraceChannel` "TraceTypeQuery1" :`bTraceComplex` true :`bIgnoreSelf` false))
        ;[1 1 1] Check if hit actor is the player/pawn
        (if _returnvalue_4
          (bind (_bblockinghit _binitialoverlap _time _distance _location _impactpoint _normal _impactnormal _physmat _hitactor _hitcomponent) (`GameplayStatics.BreakHitResult` _outhit))
          (bind _asbp_3rd_physics_player (cast `` _hitactor)
            (:`then`
              ;[1 1 1] If 'IsDead', apply force normally, else apply to 'Character Movement'
              (if (`/Game/Lessons/Lesson4/Lab4/BP_PhysicsFan.IsDead` _asbp_3rd_physics_player)
                (bind _returnvalue_5 (`KismetMathLibrary.NegateVector` _impactnormal))
                (bind _returnvalue_6 (* (`KismetMathLibrary.Normal` (+ _returnvalue _returnvalue_5)) (* (`KismetMathLibrary.Abs` (`KismetMathLibrary.Dot_VectorVector` _returnvalue _returnvalue_5)) (+ (* (- 1.0 _time) _pushforce) (* (* _pushforce 0.5) (`KismetMathLibrary.RandomFloat`))))))
                (`PrimitiveComponent.AddForceAtLocation` _hitcomponent _returnvalue_6 _impactpoint "None" :!label _label)
                (else
                  ;[1 1 1] Add force to the player
                  ; *[Note] Use add force on 'Character Movement' to simulate physics force as simulating physics on player 'Capsule' component will give control of the player to physics, disabling player movement control.
                  ; Simulating physics on 'Mesh' component will do the same and detach the mesh from the 'Capsule' component.
                  (`CharacterMovementComponent.AddForce` (`Character.CharacterMovement` _asbp_3rd_physics_player) _returnvalue_6))))
            (:`CastFailed`
              ;[1 1 1] Check for simulate physics
              (if (`SceneComponent.IsSimulatingPhysics` _hitcomponent "None")
                (goto _label)))))))))

(fn `UserConstructionScript`
  (bind _range (`self.Range`))
  (bind (_boxextent_x _boxextent_y _boxextent_z) (`KismetMathLibrary.BreakVector` (`BoxComponent.BoxExtent` _range)))
  ;[1 1 1] The Ranges set the box extent of the box collision 'Range'
  (`BoxComponent.SetBoxExtent` _range (`KismetMathLibrary.MakeVector` (`self.RangeX`) (`self.RangeY`) (`self.RangeZ`)) true)
  ;[1 1 1] Offset the box collision 'Range'
  (`SceneComponent.K2_SetRelativeLocation` _range (`KismetMathLibrary.MakeVector` 0.0 0.0 (+ _boxextent_z 20.0)) false false))