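; BP_25DCamera_Back is a follow camera for a 2.5D lesson lab that keeps a fixed offset from the player.
; BeginPlay caches the offset between its location and player character 0, then Tick moves it to the player's location plus that offset without sweeping.
; The follow applies on all three axes; the X location also saved at BeginPlay is never read.
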(event `self.ReceiveBeginPlay`
  (bind _returnvalue (`self.K2_GetActorLocation`))
  (set `self.CameraXLoc` (.x _returnvalue))
  (set `self.CameraOffset` (- _returnvalue (`self.K2_GetActorLocation` (`GameplayStatics.GetPlayerCharacter` 0)))))

(event `self.ReceiveTick`
  (params (DeltaSeconds :type "Float (single-precision)"))
  (`self.K2_SetActorLocation` (+ (`self.K2_GetActorLocation` (`GameplayStatics.GetPlayerCharacter` 0)) (`self.CameraOffset`))))

(fn `UserConstructionScript`)