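; BP_Glacier is a glacier puzzle prop that melts away when its Melt event is called.
; Melt spawns a fire dust emitter at the actor, sets the Melting flag and starts a timer that destroys the actor five seconds later.
; While Melting, Tick sinks the actor with a frame-rate-dependent AddActorLocalTransform, whose delta also carries a Z squash that this node ignores.
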(event `Melt`
  ;[1 1 1] Set Melting
  (`GameplayStatics.SpawnEmitterAtLocation` "/Game/Effects/Particles/Dust/P__Fire_Dust.P__Fire_Dust" (`self.K2_GetActorLocation`))
  (set `self.Melting` true)
  (`KismetSystemLibrary.K2_SetTimerDelegate` (delegate `Destroy Actor`) 5.0))

(event `Destroy Actor`
  ;[1 1 1] Set Melting
  (`self.K2_DestroyActor`))

(event `self.ReceiveTick`
  (params (DeltaSeconds :type "Float (single-precision)"))
  ;[1 1 1] Melting Animation
  (if (`self.Melting`)
    (`self.K2_AddActorLocalTransform` (`KismetMathLibrary.MakeTransform` (0.0 0.0 -1.0) (struct) (1.0 1.0 0.9)))))

(fn `UserConstructionScript`)