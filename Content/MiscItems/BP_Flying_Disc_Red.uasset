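; Red flying disc target that costs the player score when shot.
; On a hit by a BP_Bullet it destroys the bullet, spawns a neon explosion and laser sound at the disc, calls DecreaseScore on the BP_Sniper player, then destroys itself.
; BeginPlay starts a short delay that removes the disc automatically if it is not shot.
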(event `self.Box.OnComponentBeginOverlap`
  (params (OverlappedComponent :type "PrimitiveComponent Object Reference") (OtherActor :type "Actor Object Reference") (OtherComp :type "PrimitiveComponent Object Reference") (OtherBodyIndex :type Integer) (bFromSweep :type Boolean) (SweepResult :type "HitResult Structure (by ref)")))

(event `self.ReceiveHit`
  (params (MyComp :type "PrimitiveComponent Object Reference") (Other :type "Actor Object Reference") (OtherComp :type "PrimitiveComponent Object Reference") (bSelfMoved :type Boolean) (HitLocation :type "Vector Structure") (HitNormal :type "Vector Structure") (NormalImpulse :type "Vector Structure") (Hit :type "HitResult Structure (by ref)"))
  (bind _returnvalue (`SceneComponent.K2_GetComponentLocation` (`self.Disc`)))
  (bind _asbp_bullet (cast `/Game/MiscItems/BP_Bullet` Other))
  (`self.K2_DestroyActor` _asbp_bullet)
  (`GameplayStatics.SpawnEmitterAtLocation` "/Game/Effects/Particles/Explosion/P_NeonExplosion.P_NeonExplosion" _returnvalue)
  (`GameplayStatics.SpawnSoundAtLocation` "/Game/Audio/SoundWaves/Effect/SW_Laser_3.SW_Laser_3" _returnvalue (struct) 1.0 1.0 0.0 null null)
  (bind _asbp_sniper (cast `/Game/MiscItems/BP_Sniper` (`GameplayStatics.GetPlayerCharacter` 0)))
  (`/Game/MiscItems/BP_Sniper.Decrease Score` _asbp_sniper)
  (`self.K2_DestroyActor`))

(event `self.ReceiveBeginPlay`
  (`KismetSystemLibrary.Delay` 3.0)
  (`self.K2_DestroyActor`))

(fn `UserConstructionScript`)