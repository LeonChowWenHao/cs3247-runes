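; BP_Disc_Thrower is a spawner that launches flying discs along its forward vector during the first 30 seconds of game time.
; After a short random startup delay, a timer with looping set by TimeUp calls SpawnDisc.
; Each call spawns a regular or, less often, red disc at a random offset from the Box and applies a random-strength impulse.
; Past the limit it only clears TimeUp, without clearing the timer.
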(event `self.ReceiveBeginPlay`
  (`KismetSystemLibrary.Delay` (`KismetMathLibrary.RandomFloatInRange` 0.2 0.6))
  (`KismetSystemLibrary.K2_SetTimerDelegate` (delegate `Spawn Disc`) 3.0 (`self.TimeUp`)))

(event `Spawn Disc`
  (bind _returnvalue (* (`self.GetActorForwardVector`) (`KismetMathLibrary.RandomFloatInRange` 1500.0 2500.0)))
  (bind _returnvalue_2 (`KismetMathLibrary.MakeTransform` (+ (`SceneComponent.K2_GetComponentLocation` (`self.Box`)) (`KismetMathLibrary.MakeVector` 200.0 (`KismetMathLibrary.RandomFloatInRange` -200.0 200.0) (`KismetMathLibrary.RandomFloatInRange` -500.0 500.0))) (`SceneComponent.K2_GetComponentRotation` (`self.Box`))))
  (if (<= (`GameplayStatics.GetTimeSeconds`) 30.0)
    (if (<= (`KismetMathLibrary.RandomInteger` 100) 70)
      (bind _returnvalue_3 (`|SpawnActorFromClass` "/Game/MiscItems/BP_Flying_Disc.BP_Flying_Disc_C" _returnvalue_2 "Undefined" "OverrideRootScale" null null))
      (`PrimitiveComponent.AddImpulse` (`/Game/MiscItems/BP_Flying_Disc.Disc` _returnvalue_3) _returnvalue "None" false)
      (else
        (bind _returnvalue_4 (`|SpawnActorFromClass` "/Game/MiscItems/BP_Flying_Disc_Red.BP_Flying_Disc_Red_C" _returnvalue_2 "Undefined" "OverrideRootScale" null null))
        (`PrimitiveComponent.AddImpulse` (`/Game/MiscItems/BP_Flying_Disc_Red.Disc` _returnvalue_4) _returnvalue "None" false)))
    (else
      (set `self.TimeUp` false))))

(event `self.ReceiveTick`
  (params (DeltaSeconds :type "Float (single-precision)")))

(fn `UserConstructionScript`)